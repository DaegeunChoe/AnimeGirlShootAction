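; GA_Sprint is the Gameplay Ability for character sprinting.
; On activation it commits, applies a speed-up effect and starts a looping timer that re-commits every tick, so cost is paid continuously until a commit fails.
; On any end, including a failed first commit, it removes the speed-up, clears the timer and applies a stamina exhaustion effect.
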(event Custom|CustomEvent
  (bind _returnvalue (Ability|CommitAbility))
  (if (not _returnvalue)
    (Ability|EndAbility)))

(event Ability|EventActivateAbility
  (bind _returnvalue (Ability|CommitAbility))
  (if _returnvalue
    (bind _returnvalue_2 (Ability|ApplyGameplayEffectToOwner "/Game/AnimeGame/Bluepirnts/Character/GAS/Effects/GE_SprintSpeedUp.GE_SprintSpeedUp_C"))
    (Variables|Default|SetSpeedUpHandle _returnvalue_2)
    (bind _returnvalue_3 (Utilities|Time|SetTimerbyEvent (delegate Custom|CustomEvent) 0.1 true))
    (Variables|Default|SetTimerHandle _returnvalue_3)
    (else
      (Ability|EndAbility))))

(event Ability|EventOnEndAbility
  (params (bWasCancelled :type Boolean))
  (Ability|RemoveGameplayEffectFromOwnerWithHandle (Variables|Default|GetSpeedUpHandle))
  (Utilities|Time|ClearandInvalidateTimerbyHandle (Variables|Default|GetTimerHandle))
  (Ability|ApplyGameplayEffectToOwner "/Game/AnimeGame/Bluepirnts/Character/GAS/Effects/GE_StaminaExhaustion.GE_StaminaExhaustion_C"))