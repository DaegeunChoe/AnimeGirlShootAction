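; GA_RestoreStamina is a Gameplay Ability that regenerates the owner's stamina over time.
; On activation it stores a fast looping timer and prints a debug message.
; Each tick applies GE_RestoreStamina to the owner unless the avatar's Ability System Component has the sprint or stamina exhaustion tag.
; The graph never calls EndAbility or clears the timer.
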(event Custom|CustomEvent
  (if (not (GameplayTags|HasAnyMatchingGameplayTags (Ability|GetAbilitySystemComponent (Ability|GetAvatarActorfromActorInfo)) (GameplayTags|MakeGameplayTagContainerfromArray (Utilities|Array|MakeArray "(TagName=\"Ability.Sprint\")" "(TagName=\"Passive.Stamina.Exhaustion\")"))))
    (Ability|ApplyGameplayEffectToOwner "/Game/AnimeGame/Bluepirnts/Character/GAS/Effects/GE_RestoreStamina.GE_RestoreStamina_C")))

(event Ability|EventActivateAbility
  (bind _returnvalue (Utilities|Time|SetTimerbyEvent (delegate Custom|CustomEvent) 0.1 true))
  (Variables|Default|SetTimerHandle _returnvalue)
  (Development|PrintString "Hello"))

(event Ability|EventOnEndAbility
  (params (bWasCancelled :type Boolean)))